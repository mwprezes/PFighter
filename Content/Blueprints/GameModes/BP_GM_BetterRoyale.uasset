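; Game mode for Better Royale, a points race between lobby characters where reaching the points target wins.
; After login and a short delay, it initializes each lobby character with an ID, the default camera and its selected character from the game instance.
; CheckVictory bubble-sorts players by ascending points, then triggers fireworks for the winner once.
; Tick prints every player's score on screen for debugging.
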(event Custom|CheckVictory
  (params (Points :type Integer) (Who :type BP%20Lobby%20Character%20Base%20Object%20Reference%20%28by%20ref%29))
  (CallFunction|SortPlayersbyPoints)
  (if (>= Points (Variables|Default|GetPointsToVictory))
    (Utilities|FlowControl|DoOnce false
      (:Completed
        (CallFunction|Victory Who)
        (for _array_element (Variables|Default|GetPlayers)
          (Development|PrintString (Utilities|GetDisplayName _array_element) true true "(R=1.000000,G=0.170947,B=0.000000,A=1.000000)")
          (bind _asbp_lobby_character_base (Utilities|Casting|CastToBP_LobbyCharacterBase _array_element))
          (Development|PrintString (Utilities|String|Append " Points: " (Utilities|String|ToString(Integer) (Variables|/Game/Blueprints/Pawns/BP_LobbyCharacterBase.BP_LobbyCharacterBase_C|GetPoints _asbp_lobby_character_base))) true true "(R=1.000000,G=0.170947,B=0.000000,A=1.000000)"))))))

(event Custom|Victory
  (params (WhoWon :type BP%20Lobby%20Character%20Base%20Object%20Reference%20%28by%20ref%29))
  (Development|PrintString (Utilities|String|Append (Utilities|GetDisplayName WhoWon) " WON!") true true "(R=0.049157,G=1.000000,B=0.000000,A=1.000000)" 5.0)
  (Default|SpawnFireworks WhoWon))

(event Custom|DebugPoints
  (params (Test :type BP%20Lobby%20Character%20Base%20Object%20Reference)))

(event EventBeginPlay
  (bind _returnvalue (Actor|GetActorOfClass "/Script/Engine.CameraActor"))
  (Class|AutomationBlueprintFunctionLibrary|AutomationWaitforLoading)
  (Variables|Default|SetDefaultCamera _returnvalue))

(event EventTick
  (params (DeltaSeconds :type Float%20%28single-precision%29))
  (for _array_element (Variables|Default|GetPlayers)
    (Development|PrintString (Utilities|GetDisplayName _array_element) true true "(R=1.000000,G=0.170947,B=0.000000,A=1.000000)" 0.0)
    (bind _asbp_lobby_character_base (Utilities|Casting|CastToBP_LobbyCharacterBase _array_element))
    (Development|PrintString (Utilities|String|Append " Points: " (Utilities|String|ToString(Integer) (Variables|/Game/Blueprints/Pawns/BP_LobbyCharacterBase.BP_LobbyCharacterBase_C|GetPoints _asbp_lobby_character_base))) true true "(R=1.000000,G=0.170947,B=0.000000,A=1.000000)" 0.0)))

(event EventPostLogin
  (params (NewPlayer :type Player%20Controller%20Object%20Reference))
  (Utilities|FlowControl|Delay 2.0)
  (bind _outactors (Actor|GetAllActorsOfClass "/Game/Blueprints/Pawns/BP_LobbyCharacterBase.BP_LobbyCharacterBase_C"))
  (for (_array_element _array_index) _outactors
    (bind _aspfighter_game_instance (Utilities|Casting|CastToPFighterGameInstance (Game|GetGameInstance)))
    (Default|Init _array_element _array_index (Variables|Default|GetDefaultCamera))
    (Variables|/Game/Blueprints/Pawns/BP_FighterCharacterBase.BP_FighterCharacterBase_C|SetCharacterInfo _array_element (Utilities|Array|Get(acopy) (Variables|/Game/Blueprints/PFighterGameInstance.PFighterGameInstance_C|GetSelectedCharactersArray _aspfighter_game_instance) _array_index))
    (Utilities|Array|AddUnique (Variables|Default|GetPlayers) _array_element)))

(fn ConstructionScript)

(fn SortPlayersbyPoints
  (bind _players (Variables|Default|GetPlayers))
  (bind _output_get (LocalVariables|SetElements (Utilities|Array|Length _players)))
  (while (> _output_get 1)
    (bind (_array_element _array_index) (Utilities|Array|ForEachLoopwithBreak _players :!label _label)
      (:LoopBody
        (if (< (+ _array_index 1) (LocalVariables|GetElements))
          (if (> (Variables|/Game/Blueprints/Pawns/BP_LobbyCharacterBase.BP_LobbyCharacterBase_C|GetPoints _array_element) (Variables|/Game/Blueprints/Pawns/BP_LobbyCharacterBase.BP_LobbyCharacterBase_C|GetPoints (Utilities|Array|Get(acopy) _players (+ _array_index 1))))
            (Utilities|Array|Swap (Variables|Default|GetPlayers) _array_index (+ _array_index 1)))
          (else
            (goto _label Break))))
      (:Completed
        (Math|Integer|DecrementInt (LocalVariables|GetElements)))))
  (return))
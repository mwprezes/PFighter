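; Game mode for fighter matches that spawns players, assigns their selected characters and pairs them as opponents.
; PostLogin collects controllers and, after a delay, applies GameInstance character picks by join index, then enables Tick.
; Online, the server's Tick pairs adjacent controllers whenever their count is even, repeatedly setting side, opponent ID and both character infos.
; ChoosePlayerStart matches the last character of the start's tag to that of the controller's name.
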(event EventTick
  (params (DeltaSeconds :type Float%20%28single-precision%29))
  (bind _playercontrollers (Variables|Default|GetPlayerControllers))
  (bind _aspfighter_game_instance (Utilities|Casting|CastToPFighterGameInstance (Game|GetGameInstance)))
  (if (Variables|/Game/Blueprints/PFighterGameInstance.PFighterGameInstance_C|GetOnline? _aspfighter_game_instance)
    (Networking|SwitchHasAuthority
      (:Authority
        (if (== (Math|Integer|%(Integer) (Utilities|Array|Length _playercontrollers) 2) 0)
          (for (_array_element _array_index) _playercontrollers
            (if (== (Math|Integer|%(Integer) _array_index 2) 0)
              (Default|SetIsLeftSided _array_element true)
              (bind _asbp_fighter_character_base (Utilities|Casting|CastToBP_FighterCharacterBase (Pawn|GetControlledPawn _array_element)))
              (Default|SetLeftCharacterInfo _array_element (Variables|/Game/Blueprints/Pawns/BP_FighterCharacterBase.BP_FighterCharacterBase_C|GetCharacterInfo _asbp_fighter_character_base))
              (if (Utilities|Array|IsValidIndex _playercontrollers (+ _array_index 1))
                (Default|SetOpponentID _array_element (+ _array_index 1))
                (bind _asbp_fighter_character_base_2 (Utilities|Casting|CastToBP_FighterCharacterBase (Pawn|GetControlledPawn (Utilities|Array|Get(acopy) _playercontrollers (+ _array_index 1)))))
                (Default|SetRightCharacterInfo _array_element (Variables|/Game/Blueprints/Pawns/BP_FighterCharacterBase.BP_FighterCharacterBase_C|GetCharacterInfo _asbp_fighter_character_base_2)))
              (else
                (Default|SetIsLeftSided _array_element false)
                (bind _asbp_fighter_character_base_3 (Utilities|Casting|CastToBP_FighterCharacterBase (Pawn|GetControlledPawn _array_element)))
                (Default|SetRightCharacterInfo _array_element (Variables|/Game/Blueprints/Pawns/BP_FighterCharacterBase.BP_FighterCharacterBase_C|GetCharacterInfo _asbp_fighter_character_base_3))
                (if (Utilities|Array|IsValidIndex _playercontrollers (- _array_index 1))
                  (Default|SetOpponentID _array_element (- _array_index 1))
                  (bind _asbp_fighter_character_base_4 (Utilities|Casting|CastToBP_FighterCharacterBase (Pawn|GetControlledPawn (Utilities|Array|Get(acopy) _playercontrollers (- _array_index 1)))))
                  (Default|SetLeftCharacterInfo _array_element (Variables|/Game/Blueprints/Pawns/BP_FighterCharacterBase.BP_FighterCharacterBase_C|GetCharacterInfo _asbp_fighter_character_base_4)))))))))))

(event EventPostLogin
  (params (NewPlayer :type Player%20Controller%20Object%20Reference))
  (bind _playercontrollers (Variables|Default|GetPlayerControllers))
  (bind _asfighter_controller (Utilities|Casting|CastToFighterController NewPlayer))
  (Utilities|Array|AddUnique _playercontrollers _asfighter_controller)
  (Utilities|FlowControl|Delay 5.0)
  (bind _aspfighter_game_instance (Utilities|Casting|CastToPFighterGameInstance (Game|GetGameInstance)))
  (for (_array_element _array_index) _playercontrollers
    (bind _asbp_fighter_character_base (Utilities|Casting|CastToBP_FighterCharacterBase (Pawn|GetControlledPawn _array_element)))
    (Default|SetCharacterInfo _asbp_fighter_character_base (Utilities|Array|Get(acopy) (Variables|/Game/Blueprints/PFighterGameInstance.PFighterGameInstance_C|GetSelectedCharactersArray _aspfighter_game_instance) _array_index) _array_index)
    (Variables|/Game/Blueprints/Pawns/BP_FighterCharacterBase.BP_FighterCharacterBase_C|SetCharacterInfo _asbp_fighter_character_base (Utilities|Array|Get(acopy) (Variables|/Game/Blueprints/PFighterGameInstance.PFighterGameInstance_C|GetSelectedCharactersArray _aspfighter_game_instance) _array_index)))
  (Actor|Tick|SetActorTickEnabled true))

(fn ConstructionScript)

(fn ChoosePlayerStart
  (params (Player :type Controller%20Object%20Reference))
  (bind _returnvalue (Utilities|GetObjectName Player))
  (bind _outactors (Actor|GetAllActorsOfClass "/Script/Engine.PlayerStart"))
  (bind _array_element (Utilities|Array|ForEachLoopwithBreak _outactors :!label _label)
    (:LoopBody
      (if (Utilities|Enum|Equal(Enum) (Utilities|String|GetSubstring (Utilities|String|ToString(Name) (Variables|/Script/Engine.PlayerStart|GetPlayerStartTag _array_element)) (- (Utilities|String|Len (Utilities|String|ToString(Name) (Variables|/Script/Engine.PlayerStart|GetPlayerStartTag _array_element))) 1)) (Utilities|String|GetSubstring _returnvalue (- (Utilities|String|Len _returnvalue) 1)))
        (LocalVariables|SetPlayerStart _array_element)
        (goto _label Break)))
    (:Completed
      (return (LocalVariables|GetPlayerStart)))))
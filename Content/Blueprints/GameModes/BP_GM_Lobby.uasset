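; Lobby game mode that holds players in character selection until all are ready, then starts the match.
; PostLogin collects each LobbyPlayerController, and Tick polls their ready flags once at least two have joined.
; Ready players' character info is written by index into the PFighterGameInstance.
; When all are ready, it stores the player count, closes each selection screen's media player and launches the hard-coded Map_BR_00 through the game instance.
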(event EventPostLogin
  (params (NewPlayer :type Player%20Controller%20Object%20Reference))
  (bind _aslobby_player_controller (Utilities|Casting|CastToLobbyPlayerController NewPlayer))
  (Utilities|Array|AddUnique (Variables|Default|GetPlayerControllers) _aslobby_player_controller))

(event EventTick
  (params (DeltaSeconds :type Float%20%28single-precision%29))
  (bind _playercontrollers (Variables|Default|GetPlayerControllers))
  (if (> (Utilities|Array|Length _playercontrollers) 1)
    (Variables|Default|SetAllPlayersReady? true)
    (bind (_array_element _array_index) (Utilities|Array|ForEachLoopwithBreak _playercontrollers :!label _label)
      (:LoopBody
        (Utilities|IsValid _array_element
          (:Is%20Valid
            (if (Variables|/Game/Blueprints/Actors/LobbyPlayerController.LobbyPlayerController_C|GetIsReady _array_element)
              (bind _aspfighter_game_instance (Utilities|Casting|CastToPFighterGameInstance (Game|GetGameInstance)))
              (Utilities|Array|SetArrayElem (Variables|/Game/Blueprints/PFighterGameInstance.PFighterGameInstance_C|GetSelectedCharactersArray _aspfighter_game_instance) _array_index (Variables|/Game/Blueprints/Actors/LobbyPlayerController.LobbyPlayerController_C|GetCharacterInfo _array_element))
              (else
                (Variables|Default|SetAllPlayersReady? false)
                (goto _label Break))))))
      (:Completed
        (if (Variables|Default|GetAllPlayersReady?)
          (bind _aspfighter_game_instance_2 (Utilities|Casting|CastToPFighterGameInstance (Game|GetGameInstance)))
          (bind _output_get (Variables|/Game/Blueprints/PFighterGameInstance.PFighterGameInstance_C|SetNumberOfPlayers _aspfighter_game_instance_2 (Utilities|Array|Length _playercontrollers)))
          (Development|PrintString (Utilities|String|ToString(Integer) _output_get))
          (for _array_element_2 _playercontrollers
            (Media|MediaPlayer|Close (Variables|/Game/Blueprints/UI/MainMenu/UI_CharacterSelection.UI_CharacterSelection_C|GetMediaPlayerRef (Variables|/Game/Blueprints/Actors/LobbyPlayerController.LobbyPlayerController_C|GetCharacterSelectionReference _array_element_2)) :!class /Script/MediaAssets.MediaPlayer))
          (Default|LaunchGame _aspfighter_game_instance_2 "/Game/Maps/Map_BR_00"))))))

(fn ConstructionScript)
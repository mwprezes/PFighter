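; Base character for a networked fighting game, handling camera setup, punch and kick inputs, and a blocking flag.
; Q triggers the HUD punch combo and hits other fighters overlapping PunchCollider, while E only triggers the HUD kick combo.
; Each hit lowers the target's HP and raises the attacker's ultra points through the stats component, branching on authority between all-client and server calls.
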(event Custom|Init
  (params (PlayerID :type Integer) (Camera :type Camera%20Actor%20Object%20Reference))
  ;[1 1 1] Init
  (Game|Player|SetViewTargetwithBlend (Game|GetPlayerController PlayerID) Camera 0.0 "VTBlend_Linear" 0.0 false))

(event Custom|PunchEnemy
  (bind _bp_fightercharacterstats (Variables|Default|GetBP_FighterCharacterStats))
  (for _array_element (Collision|GetOverlappingActors (Variables|Default|GetPunchCollider) "BP_FighterCharacterBase_C" :!class /Script/Engine.PrimitiveComponent)
    (if (!= _array_element self)
      (bind _asbp_fighter_character_base (Utilities|Casting|CastToBP_FighterCharacterBase _array_element))
      (Networking|SwitchHasAuthority
        (:Authority
          (Default|DecreaseHPonAllClient (Variables|BP_FighterCharacterBase_C|GetBP_FighterCharacterStats _asbp_fighter_character_base) 1.0)
          (Default|IncreaseUltraPointsonAllClient (Variables|Default|GetBP_FighterCharacterStats) 2.0))
        (:Remote
          (Default|DecreaseHPonServer (Variables|Default|GetBP_FighterCharacterStats) (Variables|BP_FighterCharacterBase_C|GetBP_FighterCharacterStats _asbp_fighter_character_base) 1.0)
          (Default|IncreaseUltraPointsonServer _bp_fightercharacterstats _bp_fightercharacterstats 2.0))))))

(event EventBlock
  (Variables|Default|SetbIsBlocking true))

(event EventUnBlock
  (Variables|Default|SetbIsBlocking false))

(event Input|KeyboardEvents|Q
  (params (Key :type Key%20Structure :default "None"))
  (bind _fighterhudreference (Variables|Default|GetFighterHudReference))
  (:Pressed
    (Utilities|IsValid _fighterhudreference
      (:Is%20Valid
        (Default|PunchCombo _fighterhudreference)
        (CallFunction|PunchEnemy)))))

(event Input|KeyboardEvents|E
  (params (Key :type Key%20Structure :default "None"))
  (bind _fighterhudreference (Variables|Default|GetFighterHudReference))
  (:Pressed
    (Utilities|IsValid _fighterhudreference
      (:Is%20Valid
        (Default|KickCombo _fighterhudreference)))))

(fn ConstructionScript)
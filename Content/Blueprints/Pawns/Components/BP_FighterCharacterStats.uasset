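; Fighter character stats component that tracks HP, Super points and Ultra points, with functions that clamp changes to a zero floor or 100 cap.
; A looping one-second timer started on BeginPlay adds Super points locally.
; OnServer events relay HP damage to a target, and Super or Ultra gains, through OnAllClient events that apply the change.
; RepNotify handlers are empty stubs, and timed Ultra-mode logic is disconnected.
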(event Custom|DecreaseHP_OnAllClient
  (params (DecreaseValue :type Float%20%28single-precision%29))
  (CallFunction|DecreaseHP DecreaseValue))

(event Custom|UltraEvent)

(event Custom|IncreaseSuperPointsEvent
  (CallFunction|IncreaseSuperPoints 1.0))

(event Custom|DecreaseHP_OnServer
  (params (Target :type Self%20Object%20Reference) (DecreaseValue :type Float%20%28single-precision%29))
  (CallFunction|DecreaseHPonAllClient Target DecreaseValue))

(event Custom|IncreaseUltraPoints_OnServer
  (params (IncreaseValue :type Float%20%28single-precision%29))
  (CallFunction|IncreaseUltraPointsonAllClient IncreaseValue))

(event Custom|IncreaseUltraPoints_OnAllClient
  (params (IncreaseValue :type Float%20%28single-precision%29))
  (CallFunction|IncreaseUltraPoints IncreaseValue))

(event Custom|IncreaseSuperPoints_OnAllClient
  (params (IncreaseValue :type Float%20%28single-precision%29))
  (CallFunction|IncreaseSuperPoints IncreaseValue))

(event Custom|IncreaseSuperPoints_OnServer
  (params (IncreaseValue :type Float%20%28single-precision%29))
  (CallFunction|IncreaseSuperPointsonAllClient IncreaseValue))

(event EventBeginPlay
  (Utilities|Time|SetTimerbyFunctionName 0 "IncreaseSuperPointsEvent" 1.0 true))

(fn DecreaseHP
  (params (DecreaseValue :type Float%20%28single-precision%29))
  (LocalVariables|SetL_HP (- (Variables|Default|GetHP) DecreaseValue))
  (if (>= (LocalVariables|GetL_HP) 0.0)
    (Variables|Default|SetHP (LocalVariables|GetL_HP))
    (else
      (Variables|Default|SetHP 0.0))))

(fn IncreaseUltraPoints
  (params (IncreaseValue :type Float%20%28single-precision%29))
  (LocalVariables|SetL_UltraPoints (+ (Variables|Default|GetUltraPoints) IncreaseValue))
  (if (< (LocalVariables|GetL_UltraPoints) 1e+02)
    (Variables|Default|SetUltraPoints (LocalVariables|GetL_UltraPoints))
    (else
      (Variables|Default|SetUltraPoints 1e+02))))

(fn DecreaseUltraPoints
  (params (DecreaseValue :type Float%20%28single-precision%29))
  (LocalVariables|SetL_UltraPoints (- (Variables|Default|GetUltraPoints) DecreaseValue))
  (if (>= (LocalVariables|GetL_UltraPoints) 0.0)
    (Variables|Default|SetUltraPoints (LocalVariables|GetL_UltraPoints))
    (else
      (Variables|Default|SetUltraPoints 0.0))))

(fn IncreaseSuperPoints
  (params (IncreaseValue :type Float%20%28single-precision%29))
  (LocalVariables|SetL_SuperPoints (+ (Variables|Default|GetSuperPoints) IncreaseValue))
  (if (< (LocalVariables|GetL_SuperPoints) 1e+02)
    (Variables|Default|SetSuperPoints (LocalVariables|GetL_SuperPoints))
    (else
      (Variables|Default|SetSuperPoints 1e+02))))

(fn OnRepHP)

(fn OnRepUltraPoints)

(fn OnRepSuperPoints)

(fn DecreaseSuperPoints
  (params (DecreaseValue :type Float%20%28single-precision%29))
  (LocalVariables|SetL_SuperPoints (- (Variables|Default|GetSuperPoints) DecreaseValue))
  (if (>= (LocalVariables|GetL_SuperPoints) 0.0)
    (Variables|Default|SetSuperPoints (LocalVariables|GetL_SuperPoints))
    (else
      (Variables|Default|SetSuperPoints 0.0))))
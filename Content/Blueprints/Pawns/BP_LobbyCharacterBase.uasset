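; Base lobby character that can punch other characters, credit points for knockouts and respawn at player starts.
; A punch marks overlapping characters with the puncher as their Bully and launches them on the server along the puncher's forward Y axis plus slight lift.
; Server-side respawn awards the Bully a point, shuffles player starts, sphere-traces for one free of lobby characters, clears the Bully and teleports the character there.
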(event Custom|GettingPushed
  (params (PushVector :type Vector) (Actor :type BP%20Lobby%20Character%20Base%20Object%20Reference))
  ;[1 1 1] Punching
  (Networking|SwitchHasAuthority
    (:Authority
      (Character|LaunchCharacter Actor PushVector false false))))

(event Custom|PushEnemy
  ;[1 1 1] Punching
  (for _array_element (Collision|GetOverlappingActors (Variables|Default|GetPushCollider) "BP_LobbyCharacterBase_C" :!class /Script/Engine.PrimitiveComponent)
    (if (!= _array_element self)
      (bind _asbp_lobby_character_base (Utilities|Casting|CastToBP_LobbyCharacterBase _array_element))
      (Variables|BP_LobbyCharacterBase_C|SetBully _asbp_lobby_character_base self)
      (CallFunction|GettingPushed (Math|Vector|MakeVector 0.0 (.y (* (Transformation|GetActorForwardVector) (Variables|Default|GetPunchForce))) 15.0) _asbp_lobby_character_base))))

(event Custom|RespawnPlayer
  (params (Actor :type BP%20Lobby%20Character%20Base%20Object%20Reference))
  (bind _spawnpointind (Variables|Default|GetSpawnPointInd))
  ;[1 1 1] Respawning
  (Networking|SwitchHasAuthority
    (:Authority
      (bind _bully (Variables|BP_LobbyCharacterBase_C|GetBully Actor)
        (:then
          (bind _result (Math|Integer|IncrementInt (Variables|BP_LobbyCharacterBase_C|GetPoints _bully))
            (:%20%20
              (Rendering|Components|TextRender|SetText (Variables|BP_LobbyCharacterBase_C|GetTestingPoints Actor) (Utilities|Text|ToText(Integer) _result)))))
        (:else
          _))
      (bind _outactors (Actor|GetAllActorsOfClass "/Script/Engine.PlayerStart"))
      (bind _index (Utilities|FlowControl|ForLoopwithBreak 0 (- (Utilities|Array|Length _outactors) 1))
        (:LoopBody
          (Utilities|Array|Add _spawnpointind _index))
        (:Completed
          (Utilities|Array|Shuffle _spawnpointind)
          (bind _array_element (Utilities|Array|ForEachLoopwithBreak _spawnpointind :!label _label)
            (:LoopBody
              (bind _output_get (Variables|Default|SetRespLocation (Transformation|GetActorLocation (Utilities|Array|Get(acopy) _outactors _array_element))))
              (bind _outhit (Collision|SphereTraceForObjects _output_get (- _output_get 1.0) 1e+02 (Utilities|Array|MakeArray "ObjectTypeQuery3") false _outactors "ForDuration"))
              (Utilities|Casting|CastToBP_LobbyCharacterBase (.HitActor (Collision|BreakHitResult _outhit))
                (:CastFailed
                  (goto _label Break))))
            (:Completed
              (Variables|BP_LobbyCharacterBase_C|SetBully Actor 0)
              (Transformation|SetActorLocation Actor (Variables|Default|GetRespLocation) false true))))))))

(event EventBeginPlay
  (|CallParentFunction)
  (Variables|Default|SetbCanMoveInAir true))

(fn ConstructionScript)
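; BP_FighterPawnBase is a fighter pawn base Blueprint that serves as a placeholder for a fighting character's controls.
; It defines events for horizontal movement, jump, crouch, punch, kick, block, special and ultimate moves.
; Each event only prints debug text, either the axis value or the action name, with no movement or combat logic.
; The construction script is empty.
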(event EventUltimate
  (Development|PrintString "Ultimate"))

(event EventJump
  (Development|PrintString "Jump"))

(event EventMoveRight
  (params (AxisValue :type Float%20%28single-precision%29))
  (Development|PrintString (Utilities|String|ToString(Float) AxisValue) true true "(R=0.000000,G=0.660000,B=1.000000,A=1.000000)" 0.0))

(event EventPunch
  (Development|PrintString "Punch"))

(event EventKick
  (Development|PrintString "Kick"))

(event EventCrouch
  (Development|PrintString "Crouch"))

(event EventBlock
  (Development|PrintString "Block"))

(event EventSpecial
  (Development|PrintString "Special"))

(fn ConstructionScript)
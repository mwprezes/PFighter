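; Player controller for the main menu that creates the menu widget and routes menu navigation input to it.
; On BeginPlay it creates UI_MainMenu, adds it to the player screen, sets game-and-UI input mode focused on it and shows the mouse cursor.
; Directional, confirm and back input actions call matching functions on the stored widget reference, leaving the navigation logic to the widget.
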(event EventBeginPlay
  (bind _self self)
  (bind _returnvalue (UserInterface|CreateWidget "/Game/Blueprints/UI/MainMenu/UI_MainMenu.UI_MainMenu_C" _self))
  (bind _output_get (Variables|Default|SetMainMenuReference _returnvalue))
  (Utilities|IsValid _output_get
    (:Is%20Valid
      (UserInterface|Viewport|AddtoPlayerScreen _output_get)
      (Input|SetInputModeGameandUI _self _returnvalue "DoNotLock" true)
      (Variables|/Script/Engine.PlayerController|SetbShowMouseCursor _self true))))

(event Input|ActionEvents|InputActionUI_Right
  (params (Key :type Key%20Structure :default "None"))
  (:Pressed
    (Default|UIRight (Variables|Default|GetMainMenuReference))))

(event Input|ActionEvents|InputActionUI_Left
  (params (Key :type Key%20Structure :default "None"))
  (:Pressed
    (Default|UILeft (Variables|Default|GetMainMenuReference))))

(event Input|ActionEvents|InputActionUI_Up
  (params (Key :type Key%20Structure :default "None"))
  (:Pressed
    (Default|UIUp (Variables|Default|GetMainMenuReference))))

(event Input|ActionEvents|InputActionUI_Down
  (params (Key :type Key%20Structure :default "None"))
  (:Pressed
    (Default|UIDown (Variables|Default|GetMainMenuReference))))

(event Input|ActionEvents|InputActionUI_Confirm
  (params (Key :type Key%20Structure :default "None"))
  (:Pressed
    (Default|UIConfirm (Variables|Default|GetMainMenuReference))))

(event Input|ActionEvents|InputActionUI_Back
  (params (Key :type Key%20Structure :default "None"))
  (:Pressed
    (Default|UIBack (Variables|Default|GetMainMenuReference))))

(fn ConstructionScript)
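; Lobby player controller that drives character selection and records the player's choice.
; On BeginPlay, the local controller creates the character selection widget on the player's screen and enables Game and UI input with a visible cursor.
; UI input actions forward to that widget to cycle characters and attacks or confirm the pick.
; SetCharacterInfo stores the chosen info and passes it to SetInfo, which stores it and marks the player ready.
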(event Custom|SetInfo
  (params (CharacterInfo :type ST%20Character%20Info%20Structure))
  (Variables|Default|SetCharacterInfo CharacterInfo)
  (Variables|Default|SetIsReady true))

(event Custom|SetCharacterInfo
  (params (CharacterInfo :type ST%20Character%20Info%20Structure))
  (bind _output_get (Variables|Default|SetCharacterInfo CharacterInfo))
  (CallFunction|SetInfo _output_get))

(event EventBeginPlay
  (bind _self self)
  (if (Pawn|IsLocalController)
    (bind _returnvalue (UserInterface|CreateWidget "/Game/Blueprints/UI/MainMenu/UI_CharacterSelection.UI_CharacterSelection_C" _self))
    (Variables|Default|SetCharacterSelectionReference _returnvalue)
    (Utilities|IsValid _returnvalue
      (:Is%20Valid
        (UserInterface|Viewport|AddtoPlayerScreen _returnvalue)
        (Input|SetInputModeGameandUI _self 0 "DoNotLock" true)
        (Variables|/Script/Engine.PlayerController|SetbShowMouseCursor _self true)))))

(event Input|ActionEvents|InputActionUI_Right
  (params (Key :type Key%20Structure :default "None"))
  (bind _characterselectionreference (Variables|Default|GetCharacterSelectionReference))
  (:Pressed
    (Utilities|IsValid _characterselectionreference
      (:Is%20Valid
        (Default|IncreaseCharacterIndex _characterselectionreference)))))

(event Input|ActionEvents|InputActionUI_Left
  (params (Key :type Key%20Structure :default "None"))
  (bind _characterselectionreference (Variables|Default|GetCharacterSelectionReference))
  (:Pressed
    (Utilities|IsValid _characterselectionreference
      (:Is%20Valid
        (Default|DecreaseCharacterIndex _characterselectionreference)))))

(event Input|ActionEvents|InputActionUI_Up
  (params (Key :type Key%20Structure :default "None"))
  (bind _characterselectionreference (Variables|Default|GetCharacterSelectionReference))
  (:Pressed
    (Utilities|IsValid _characterselectionreference
      (:Is%20Valid
        (Default|DecreaseAttackIndex _characterselectionreference)))))

(event Input|ActionEvents|InputActionUI_Down
  (params (Key :type Key%20Structure :default "None"))
  (bind _characterselectionreference (Variables|Default|GetCharacterSelectionReference))
  (:Pressed
    (Utilities|IsValid _characterselectionreference
      (:Is%20Valid
        (Default|IncreaseAttackIndex _characterselectionreference)))))

(event Input|ActionEvents|InputActionUI_Confirm
  (params (Key :type Key%20Structure :default "None"))
  (bind _characterselectionreference (Variables|Default|GetCharacterSelectionReference))
  (:Pressed
    (Utilities|IsValid _characterselectionreference
      (:Is%20Valid
        (Default|SelectCharacter _characterselectionreference)))))

(fn ConstructionScript)
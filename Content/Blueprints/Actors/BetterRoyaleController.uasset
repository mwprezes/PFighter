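; BetterRoyaleController is a controller that sets up and updates the player's HUD for the Better Royale mode.
; InitHUD creates either the Better Royale HUD or the main game HUD based on a mode flag, stores the reference and adds it to the player screen.
; Update events forward player points, big and small icons, and the player count to the Better Royale HUD; only the points update checks that the HUD is valid.
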(event Custom|InitHUD
  (params (BetterRoyaleMode? :type Boolean))
  (if BetterRoyaleMode?
    (bind _returnvalue (UserInterface|CreateWidget "/Game/Blueprints/UI/BetterRoyaleHUD/UI_BetterRoyale_HUD.UI_BetterRoyale_HUD_C" self))
    (Variables|Default|SetBetterRoyaleHUDReference _returnvalue)
    (Utilities|IsValid _returnvalue
      (:Is%20Valid
        (UserInterface|Viewport|AddtoPlayerScreen _returnvalue)))
    (else
      (bind _returnvalue_2 (UserInterface|CreateWidget "/Game/Blueprints/UI/GameHUD/GameHUD_Main.GameHUD_Main_C" self))
      (Variables|Default|SetFighterHudReference _returnvalue_2)
      (Utilities|IsValid _returnvalue_2
        (:Is%20Valid
          (UserInterface|Viewport|AddtoPlayerScreen _returnvalue_2))))))

(event Custom|UpdateNumberOfPlayersInBetterRoyale
  (params (NumberOfPlayers :type Integer))
  (Default|UpdateNumberOfPlayers (Variables|Default|GetBetterRoyaleHUDReference) NumberOfPlayers))

(event Custom|UpdatePlayersPointsInBetterRoyale
  (params (PlayersPoints :type Array%20of%20Integers) (IconBig :type Array%20of%20Texture%202D%20Object%20References) (IconSmall :type Array%20of%20Texture%202D%20Object%20References))
  (bind _betterroyalehudreference (Variables|Default|GetBetterRoyaleHUDReference))
  (Utilities|IsValid _betterroyalehudreference
    (:Is%20Valid
      (Default|UpdatePoints _betterroyalehudreference PlayersPoints IconBig IconSmall))))

(fn ConstructionScript)
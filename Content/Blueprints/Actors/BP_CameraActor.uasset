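; Shared camera actor that frames the two players of one fighting row.
; On authority BeginPlay it waits for loading, signals init complete to enable ticking, and multicasts SetView after a delay.
; SetView derives both player indices from FightingRow and blends their controllers' views to this actor.
; Tick follows the players' midpoint along Y only and scales spring arm length with their distance, within clamped limits.
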(event Custom|StartTicking
  ;[1 1 1] SetupCameraForPlayers
  (Actor|Tick|SetActorTickEnabled true))

(event Custom|MulticastSetView
  ;[1 1 1] SetupCameraForPlayers
  (CallFunction|SetView (Variables|Settings|GetFightingRow)))

(event EventBeginPlay
  ;[1 1 1] SetupCameraForPlayers
  (Networking|SwitchHasAuthority
    (:Authority
      (EventDispatchers|BindEventtoInitComplete (delegate Custom|StartTicking))
      (Class|AutomationBlueprintFunctionLibrary|AutomationWaitforLoading)
      (Utilities|FlowControl|Sequence
        (:then_0
          (Utilities|FlowControl|Delay 5.0)
          (CallFunction|MulticastSetView))
        (:then_1
          (Default|CallInitComplete))))))

(event EventTick
  (params (DeltaSeconds :type Float%20%28single-precision%29))
  (bind _returnvalue (Transformation|GetActorLocation))
  (bind _player1 (Variables|Default|GetPlayer1)
    (:then
      (bind _player2 (Variables|Default|GetPlayer2)
        (:then
          (Variables|/Script/Engine.SpringArmComponent|SetTargetArmLength (Variables|Default|GetSpringArm) (Math|Float|Clamp(Float) (/ (Math|Vector|Distance(Vector) (Transformation|GetActorLocation _player1) (Transformation|GetActorLocation _player2)) 1.5) 5e+02 1.8e+03))
          (Transformation|SetActorLocation (Math|Vector|MakeVector (.x _returnvalue) (.y (/ (+ (Transformation|GetActorLocation _player1) (Transformation|GetActorLocation _player2)) 2.0)) (.z _returnvalue)) false false))
        (:else)))
    (:else)))

(fn ConstructionScript)

(fn SetView
  (params (RowIndex :type Integer))
  (bind _returnvalue (- RowIndex 1))
  (bind _returnvalue_2 (* _returnvalue 2))
  (bind _returnvalue_3 (Game|GetPlayerCharacter _returnvalue_2))
  (bind _returnvalue_4 (+ _returnvalue_2 1))
  (bind _returnvalue_5 (Game|GetPlayerCharacter _returnvalue_4))
  (Utilities|IsValid _returnvalue_3
    (:Is%20Valid
      (Variables|Default|SetPlayer1 _returnvalue_3)
      (Game|Player|SetViewTargetwithBlend (Game|GetPlayerController _returnvalue_2) self 0.0 "VTBlend_Linear" 0.0 false)
      (Utilities|IsValid _returnvalue_5
        (:Is%20Valid
          (Variables|Default|SetPlayer2 _returnvalue_5)
          (Game|Player|SetViewTargetwithBlend (Game|GetPlayerController _returnvalue_4) self 0.0 "VTBlend_Linear" 0.0 false))))))
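; FighterController is the player controller for a fighting game, owning the local fight HUD and the selected character info.
; On BeginPlay it adds GameHUD_Main for local players and, when offline, sets left character info from the game instance's first selection.
; With a valid HUD, Q triggers its punch combo for the controller's side and the fighter pawn's punch, while E triggers only the HUD's kick combo.
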(event Custom|SetRightCharacterInfo
  (params (CharacterInfo :type ST%20Character%20Info%20Structure))
  (Variables|Default|SetRightCharacterInfo CharacterInfo))

(event Custom|SetLeftCharacterInfo
  (params (CharacterInfo :type ST%20Character%20Info%20Structure))
  (Variables|Default|SetLeftCharacterInfo CharacterInfo))

(event EventBeginPlay
  (bind _self self)
  (Utilities|FlowControl|Sequence
    (:then_0
      (if (Pawn|IsLocalController _self)
        (bind _returnvalue (UserInterface|CreateWidget "/Game/Blueprints/UI/GameHUD/GameHUD_Main.GameHUD_Main_C" _self))
        (bind _output_get (Variables|Default|SetFighterHudReference _returnvalue))
        (Utilities|IsValid _output_get
          (:Is%20Valid
            (UserInterface|Viewport|AddtoPlayerScreen _output_get)))))
    (:then_1
      (bind _aspfighter_game_instance (Utilities|Casting|CastToPFighterGameInstance (Game|GetGameInstance)))
      (if (not (Variables|/Game/Blueprints/PFighterGameInstance.PFighterGameInstance_C|GetOnline? _aspfighter_game_instance))
        (CallFunction|SetLeftCharacterInfo (Utilities|Array|Get(acopy) (Variables|/Game/Blueprints/PFighterGameInstance.PFighterGameInstance_C|GetSelectedCharactersArray _aspfighter_game_instance)))))))

(event Input|KeyboardEvents|Q
  (params (Key :type Key%20Structure :default "None"))
  (bind _fighterhudreference (Variables|Default|GetFighterHudReference))
  (:Pressed
    (Utilities|IsValid _fighterhudreference
      (:Is%20Valid
        (Default|PunchCombo _fighterhudreference (Variables|Default|GetIsLeftSided?))
        (bind _asbp_fighter_character_base (Utilities|Casting|CastToBP_FighterCharacterBase (Pawn|GetControlledPawn)))
        (Default|PunchEnemy _asbp_fighter_character_base)))))

(event Input|KeyboardEvents|E
  (params (Key :type Key%20Structure :default "None"))
  (bind _fighterhudreference (Variables|Default|GetFighterHudReference))
  (:Pressed
    (Utilities|IsValid _fighterhudreference
      (:Is%20Valid
        (Default|KickCombo _fighterhudreference (Variables|Default|GetIsLeftSided?))))))

(fn ConstructionScript)
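; BP_CharacterBase is a Character Blueprint with Punch and Kick input actions and a shared montage helper.
; Both input events currently only print the action name on press, with no animation or combat logic attached.
; TryPlayAnimMontage plays a given montage only if it is not already playing and returns whether it started playback, but neither input event calls it.
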(event Input|ActionEvents|InputActionPunch
  (params (Key :type Key%20Structure :default "None"))
  (:Pressed
    (Development|PrintString "Punch")))

(event Input|ActionEvents|InputActionKick
  (params (Key :type Key%20Structure :default "None"))
  (:Pressed
    (Development|PrintString "Kick")))

(fn ConstructionScript)

(fn TryPlayAnimMontage
  (params (Montage :type Anim%20Montage%20Object%20Reference))
  (if (Animation|Montage|MontageIsPlaying (Components|SkeletalMesh|GetAnimInstance (Variables|Character|GetMesh)) Montage)
    (return false)
    (else
      (Animation|PlayAnimMontage Montage 1.0 "None")
      (return true))))
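; Player controller that turns buffered input sequences into character moves, such as fighting-game style commands.
; On begin play it caches the controlled BP_CharacterBase; after input is buffered, and only while that character is idle, it tests each InputCommands entry in array order.
; The first command matched by InputBuffer plays the CharacterMoves montage at the same index and clears the history, so earlier entries take priority.
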(event Custom|TryBufferedMove
  ;[1 1 1] Try Buffered Move
  (bind _isidle (Default|IsIdle (Variables|Default|GetControllerCharacter)))
  (if _isidle
    (bind (_array_element _array_index) (Utilities|Array|ForEachLoopwithBreak (Variables|Default|GetInputCommands) :!label _label)
      (:LoopBody
        (bind _issuccessfull (CallFunction|TryMove (Utilities|Array|Get(acopy) (Variables|Default|GetCharacterMoves) _array_index) _array_element))
        (if _issuccessfull
          (goto _label Break))))))

(event EventBeginPlay
  ;[1 1 1] Begin Play
  (bind _asbp_character_base (Utilities|Casting|CastToBP_CharacterBase (Pawn|GetControlledPawn)))
  (Variables|Default|SetControllerCharacter _asbp_character_base))

(event EventPostBufferInput
  ;[1 1 1] Post Buffer Input
  (CallFunction|TryBufferedMove))

(fn ConstructionScript)

(fn TryMove
  (params (Montage :type Anim%20Montage%20Object%20Reference) (Command :type Input%20Command%20Object%20Reference))
  (if (Class|InputBufferComponent|MatchCommand (Variables|Default|GetInputBuffer) Command)
    (Animation|PlayAnimMontage (Variables|Default|GetControllerCharacter) Montage 1.0 "None")
    (Class|InputBufferComponent|ClearHistory (Variables|Default|GetInputBuffer))
    (return true)
    (else
      (return false))))